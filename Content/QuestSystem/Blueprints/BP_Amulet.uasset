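; BP_Amulet is a quest pickup that completes a FindAmulet quest objective when the player touches it.
; On BeginPlay it caches the level's BP_Service actor as its service manager.
; When a Player-tagged actor overlaps its sphere collision, it reads the FindAmulet row from DT_Quest and completes that quest's second objective through the manager.
; It then sets the manager's FindAmulet flag and destroys itself.
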(event `self.ReceiveBeginPlay`
  (bind _returnvalue (`GameplayStatics.GetActorOfClass` "/Game/QuestSystem/Blueprints/BP_Service.BP_Service_C"))
  (set `self.ServiceManager` _returnvalue))

(event `self.SphereCollision.OnComponentBeginOverlap`
  (params (OverlappedComponent :type "PrimitiveComponent Object Reference") (OtherActor :type "Actor Object Reference") (OtherComp :type "PrimitiveComponent Object Reference") (OtherBodyIndex :type Integer) (bFromSweep :type Boolean) (SweepResult :type "HitResult Structure (by ref)"))
  (bind _servicemanager (`self.ServiceManager`))
  (if (`self.ActorHasTag` OtherActor "Player")
    (bind _returnvalue (`|GetDataTableRow` "/Game/QuestSystem/DataTables/DT_Quest.DT_Quest" "FindAmulet")
      (:`then`
        (bind ((`QuestID_15_822500384463595D74E8C3A0EFD088AB` _questid) (`Objectives_20_897191804E9E5A681C401483E0AEB55B` _objectives)) (break `/Game/QuestSystem/Structs/S_QuestData` _returnvalue))
        (`/Game/QuestSystem/Blueprints/BP_Service.SM_CompleteObjective` _servicemanager _questid (`.ObjectiveID_5_E318AE8B44FE4C490F23A1996DC67BF0` (break `/Game/QuestSystem/Structs/S_QuestObjective` (`|GetArrayItem` _objectives 1))))
        (set `/Game/QuestSystem/Blueprints/BP_Service.FindAmulet?` true _servicemanager)
        (`self.K2_DestroyActor`)))))

(fn `UserConstructionScript`)