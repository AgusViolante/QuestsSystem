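; BP_CharacterQuest is a quest NPC that plays a line-by-line dialogue and reports quest completion.
; Each Interact advances TalkIndex and shows the next Dialogue entry in a lazily created WBP_Dialogue widget.
; An Interact after the last line removes the widget and calls NPCCompleteQuest on the BP_Service found at BeginPlay.
; A box overlap with a Player-tagged actor only prints a debug greeting, and GetHUD and GetServiceManager are empty.
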(event `self.ReceiveBeginPlay`
  (bind _returnvalue (`GameplayStatics.GetActorOfClass` "/Game/QuestSystem/Blueprints/BP_Service.BP_Service_C"))
  (set `self.ServiceManager` _returnvalue))

(event `self.Box.OnComponentBeginOverlap`
  (params (OverlappedComponent :type "PrimitiveComponent Object Reference") (OtherActor :type "Actor Object Reference") (OtherComp :type "PrimitiveComponent Object Reference") (OtherBodyIndex :type Integer) (bFromSweep :type Boolean) (SweepResult :type "HitResult Structure (by ref)"))
  (if (`self.ActorHasTag` OtherActor "Player")
    (`KismetSystemLibrary.PrintString` "Hello")))

(event `/Game/QuestSystem/Interfaces/IA_Player.Interact`
  (bind _talkindex (`self.TalkIndex`))
  (if (not (`self.FinishDialogue`))
    (`/Engine/EditorBlueprintResources/StandardMacros.IncrementInt` _talkindex
      (:`  `
        (if (<= _talkindex (`KismetArrayLibrary.Array_Length` (`self.Dialogue`)))
          (`self.WBP_DialogueREF`
            (:`then`
              _)
            (:`else`
              (bind _returnvalue (`|CreateWidget` "/Game/QuestSystem/Widgets/WBP_Dialogue.WBP_Dialogue_C"))
              (bind _output_get (set `self.WBP_DialogueREF` _returnvalue))
              (`UserWidget.AddToViewport` _output_get 0)))
          (`TextBlock.SetText` (`/Game/QuestSystem/Widgets/WBP_Dialogue.TalkText` (`self.WBP_DialogueREF`)) (`KismetTextLibrary.Conv_StringToText` (`|GetArrayItem` (`self.Dialogue`) (- (`self.TalkIndex`) 1))))
          (if (== (`self.TalkIndex`) (`KismetArrayLibrary.Array_Length` (`self.Dialogue`)))
            (set `self.FinishDialogue` true)))))
    (else
      (`Widget.RemoveFromParent` (`self.WBP_DialogueREF`))
      (`/Game/QuestSystem/Blueprints/BP_Service.NPC_CompleteQuest` (`self.ServiceManager`)))))

(fn `GetHUD`
  (returns (HUDRef :type "/Game/QuestSystem/Widgets/WBP_QuestHUD Object Reference"))
  (return null))

(fn `GetServiceManager`
  (returns (`Service Manager` :type "/Game/QuestSystem/Blueprints/BP_Service Object Reference"))
  (return null))

(fn `UserConstructionScript`)