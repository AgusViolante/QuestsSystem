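; Quest service Blueprint that acts as a facade over the quest manager, forwarding start, auto-start, objective completion, active-widget and quest-list calls.
; NPCCompleteQuest also hardcodes an NPC's amulet quest flow, starting the first DT_Quest row on first contact.
; Later calls complete FindAmulet's first or third objective depending on the FindAmulet flag.
; The final stage only prints XP rewards and sets IsCompleted inside that reward loop.
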(event `/Game/QuestSystem/Interfaces/IA_ServiceManager.SM_StartQuest`
  (params (Quest :type Name))
  (`/Game/QuestSystem/Interfaces/IA_QuestManager.QM_StartQuest` (`self.BP_QuestManager_REF`) Quest))

(event `/Game/QuestSystem/Interfaces/IA_ServiceManager.SM_CompleteObjective`
  (params (QuestID :type Name) (ObjectiveID :type Name))
  (`/Game/QuestSystem/Interfaces/IA_QuestManager.QM_CompleteObjective` (`self.BP_QuestManager_REF`) QuestID ObjectiveID))

(event `/Game/QuestSystem/Interfaces/IA_ServiceManager.SM_AutoStartQuests`
  (`/Game/QuestSystem/Interfaces/IA_QuestManager.QM_AutoStartQuests` (`self.BP_QuestManager_REF`)))

(event `/Game/QuestSystem/Interfaces/IA_ServiceManager.SM_SetActiveWidget`
  (params (Widget :type "Widget Object Reference"))
  (`/Game/QuestSystem/Interfaces/IA_QuestManager.QM_UpdateActiveWidget` (`self.BP_QuestManager_REF`) Widget))

(fn `NPC_CompleteQuest`
  (if (not (`self.IsCompleted?`))
    (if (`self.Hablo?`)
      (if (not (`self.FindAmulet?`))
        (bind _returnvalue (`|GetDataTableRow` "/Game/QuestSystem/DataTables/DT_Quest.DT_Quest" "FindAmulet")
          (:`then`
            (bind ((`QuestID_15_822500384463595D74E8C3A0EFD088AB` _questid) (`Objectives_20_897191804E9E5A681C401483E0AEB55B` _objectives)) (break `/Game/QuestSystem/Structs/S_QuestData` _returnvalue))
            (`self.SM_CompleteObjective` _questid (`.ObjectiveID_5_E318AE8B44FE4C490F23A1996DC67BF0` (break `/Game/QuestSystem/Structs/S_QuestObjective` (`|GetArrayItem` _objectives))))
            (`KismetSystemLibrary.PrintString` "Parte 2")))
        (else
          (bind _returnvalue_2 (`|GetDataTableRow` "/Game/QuestSystem/DataTables/DT_Quest.DT_Quest" "FindAmulet")
            (:`then`
              (bind ((`QuestID_15_822500384463595D74E8C3A0EFD088AB` _questid_2) (`Objectives_20_897191804E9E5A681C401483E0AEB55B` _objectives_2) (`Rewards_22_FA429F1740E8EE2A368BD4AC79BB848B` _rewards)) (break `/Game/QuestSystem/Structs/S_QuestData` _returnvalue_2))
              (`self.SM_CompleteObjective` _questid_2 (`.ObjectiveID_5_E318AE8B44FE4C490F23A1996DC67BF0` (break `/Game/QuestSystem/Structs/S_QuestObjective` (`|GetArrayItem` _objectives_2 2))))
              (for _array_element _rewards
                (`KismetSystemLibrary.PrintString` (`KismetStringLibrary.Concat_StrStr` "Ganaste:   " "XP:  " (`KismetStringLibrary.Conv_IntToString` (`.XP_6_1AF806074FC432942D4A11AB5CECE36E` (break `/Game/QuestSystem/Structs/S_Rewards` _array_element)))))
                (`KismetSystemLibrary.PrintString` "Parte 3")
                (set `self.IsCompleted?` true))))))
      (else
        (bind _outrownames (`DataTableFunctionLibrary.GetDataTableRowNames` "/Game/QuestSystem/DataTables/DT_Quest.DT_Quest"))
        (`/Game/QuestSystem/Interfaces/IA_ServiceManager.SM_StartQuest` (`|GetArrayItem` _outrownames))
        (`KismetSystemLibrary.PrintString` "tenes la mision")
        (set `self.Hablo?` true)
        (`KismetSystemLibrary.PrintString` "Parte 1")))
    (else
      (`KismetSystemLibrary.PrintString` "Ya completaste esta mision"))))

(fn `SM_GetActiveQuests`
  (returns (ActiveQuests :type "Array of /Game/QuestSystem/Structs/S_QuestData Structure"))
  (bind _activequests (message `/Game/QuestSystem/Interfaces/IA_QuestManager.QM_GetActiveQuests` (`self.BP_QuestManager_REF`)))
  (return _activequests))

(fn `SM_GetActiveWidget`
  (returns (Widget :type "Widget Object Reference"))
  (bind _widget (`/Game/QuestSystem/Interfaces/IA_QuestManager.QM_GetActiveWidget` (`self.BP_QuestManager_REF`)))
  (return _widget))

(fn `SM_GetCompletedQuests`
  (returns (CompletedQuests :type "Array of /Game/QuestSystem/Structs/S_QuestData Structure"))
  (bind _completedquests (message `/Game/QuestSystem/Interfaces/IA_QuestManager.QM_GetCompletedQuests` (`self.BP_QuestManager_REF`)))
  (return _completedquests))

(fn `UserConstructionScript`)