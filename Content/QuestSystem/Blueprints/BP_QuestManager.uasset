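; Quest manager that starts, tracks and completes quests defined in DT_Quest, including auto-start rows.
; Starting rejects active or finished non-repeatable quests, then copies the row into ActiveQuests and shows a popup.
; Completing an objective rebuilds its struct, updates QuestProgress and moves fully completed quests to CompletedQuest.
; QM-prefixed events and getters expose this, though objective update and completion-check loops return false unless the quest is first in ActiveQuests.
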(event `/Game/QuestSystem/Interfaces/IA_QuestManager.QM_StartQuest`
  (params (QuestID :type Name))
  (`self.StartQuest` QuestID))

(event `/Game/QuestSystem/Interfaces/IA_QuestManager.QM_CompleteObjective`
  (params (QuestID :type Name) (ObjectiveID :type Name))
  (bind _output (`self.CompleteObjective` QuestID ObjectiveID))
  (if _output
    (`self.CompleteQuest` QuestID)))

(event `/Game/QuestSystem/Interfaces/IA_QuestManager.QM_AutoStartQuests`
  (bind _outrownames (`DataTableFunctionLibrary.GetDataTableRowNames` "/Game/QuestSystem/DataTables/DT_Quest.DT_Quest"))
  (for _array_element _outrownames
    (bind _returnvalue (`|GetDataTableRow` "/Game/QuestSystem/DataTables/DT_Quest.DT_Quest" _array_element)
      (:`then`
        (bind ((`QuestID_15_822500384463595D74E8C3A0EFD088AB` _questid) (`AutoStart_12_943067A9438EE77023CA318B13FC3695` _autostart)) (break `/Game/QuestSystem/Structs/S_QuestData` _returnvalue))
        (if _autostart
          (`self.StartQuest` _questid))))))

(event `/Game/QuestSystem/Interfaces/IA_QuestManager.QM_UpdateActiveWidget`
  (params (Widget :type "Widget Object Reference"))
  (set `self.ActiveWidget` Widget))

(fn `CheckIfQuestHasAlready`
  (params (QuestID :type Name))
  (returns (`CanStart?` :type Boolean))
  (for _array_element (`self.CompletedQuest`)
    (bind ((`QuestID_15_822500384463595D74E8C3A0EFD088AB` _questid) (`IsRepitable_9_AD8D6185495E1891D2BDCB9137FF07FB` _isrepitable)) (break `/Game/QuestSystem/Structs/S_QuestData` _array_element))
    (if (and (== _questid QuestID) (not _isrepitable))
      (return false)))
  (for _array_element_2 (`self.ActiveQuests`)
    (if (== (`.QuestID_15_822500384463595D74E8C3A0EFD088AB` (break `/Game/QuestSystem/Structs/S_QuestData` _array_element_2)) QuestID)
      (return false)))
  (return true))

(fn `CheckQuestCompleted`
  (params (QuestID :type Name))
  (returns (`Completed?` :type Boolean))
  (for _array_element (`self.ActiveQuests`)
    (if (== (`.QuestID_15_822500384463595D74E8C3A0EFD088AB` (break `/Game/QuestSystem/Structs/S_QuestData` _array_element)) QuestID)
      (for _array_element_2 (`.Objectives_20_897191804E9E5A681C401483E0AEB55B` (break `/Game/QuestSystem/Structs/S_QuestData` _array_element))
        (if (not (`.IsCompleted_16_F1BD629D49891E8A858FFC8431AD9FC4` (break `/Game/QuestSystem/Structs/S_QuestObjective` _array_element_2)))
          (return false)))
      (return true)
      (else
        (return false)))))

(fn `CompleteObjective`
  (params (QuestID :type Name) (ObjectiveID :type Name))
  (returns (Output :type Boolean))
  (locals (TempProgress :type "Map of Name to Object Object Reference"))
  (bind (_value _returnvalue) (`BlueprintMapLibrary.Map_Find` (`local.TempProgress`) QuestID))
  (bind _completed_ (`self.UpdateObjectiveCompletion` QuestID ObjectiveID))
  (set `local.TempProgress` (`self.QuestProgress`))
  (if _returnvalue
    (bind _result (`/Engine/EditorBlueprintResources/StandardMacros.IncrementInt` _value)
      (:`  `
        (`BlueprintMapLibrary.Map_Add` (`local.TempProgress`) QuestID _result)
        (set `self.QuestProgress` (`local.TempProgress`))
        (bind _returnvalue_2 (`|GetDataTableRow` "/Game/QuestSystem/DataTables/DT_Quest.DT_Quest" QuestID)
          (:`then`
            (for _array_element (`.Objectives_20_897191804E9E5A681C401483E0AEB55B` (break `/Game/QuestSystem/Structs/S_QuestData` _returnvalue_2))
              (if (== (`.ObjectiveID_5_E318AE8B44FE4C490F23A1996DC67BF0` (break `/Game/QuestSystem/Structs/S_QuestObjective` _array_element)) (`local.ObjectiveID`))
                (bind _returnvalue_3 (`|CreateWidget` "/Game/QuestSystem/Widgets/WBP_CompletedObjective.WBP_CompletedObjective_C" null _array_element))
                (`UserWidget.AddToViewport` _returnvalue_3 0)))
            (return _completed_)))))
    (else
      (return false))))

(fn `CompleteQuest`
  (params (QuestID :type Name))
  (for _array_element (`self.ActiveQuests`)
    (if (== (`.QuestID_15_822500384463595D74E8C3A0EFD088AB` (break `/Game/QuestSystem/Structs/S_QuestData` _array_element)) QuestID)
      (bind _returnvalue (`|CreateWidget` "/Game/QuestSystem/Widgets/WBP_StartedQuest.WBP_StartedQuest_C" null _array_element))
      (`UserWidget.AddToViewport` _returnvalue 0)
      (`KismetArrayLibrary.Array_Add` (`self.CompletedQuest`) _array_element)
      (`KismetArrayLibrary.Array_RemoveItem` (`self.ActiveQuests`) _array_element)
      (`BlueprintMapLibrary.Map_Remove` (`self.QuestProgress`) QuestID)
      (return))))

(fn `QM_GetActiveQuests`
  (returns (ActiveQuests :type "Array of /Game/QuestSystem/Structs/S_QuestData Structure"))
  (return (`self.ActiveQuests`)))

(fn `QM_GetActiveWidget`
  (returns (Widget :type "Widget Object Reference"))
  (return (`self.ActiveWidget`)))

(fn `QM_GetCompletedQuests`
  (returns (CompletedQuests :type "Array of /Game/QuestSystem/Structs/S_QuestData Structure"))
  (return (`self.CompletedQuest`)))

(fn `StartQuest`
  (params (QuestID :type Name))
  (locals (TempProgress :type "Map of Name to Object Object Reference"))
  (bind _tempprogress (`local.TempProgress`))
  (bind _canstart_ (`self.CheckIfQuestHasAlready` QuestID))
  (if _canstart_
    (bind _returnvalue (`|GetDataTableRow` "/Game/QuestSystem/DataTables/DT_Quest.DT_Quest" QuestID)
      (:`then`
        (`KismetArrayLibrary.Array_Add` (`self.ActiveQuests`) _returnvalue)
        (set `local.TempProgress` (`self.QuestProgress`))
        (`BlueprintMapLibrary.Map_Add` _tempprogress QuestID)
        (set `self.QuestProgress` _tempprogress)
        (bind _returnvalue_2 (`|CreateWidget` "/Game/QuestSystem/Widgets/WBP_StartedQuest.WBP_StartedQuest_C" null _returnvalue))
        (`UserWidget.AddToViewport` _returnvalue_2 0)))))

(fn `UpdateObjectiveCompletion`
  (params (QuestID :type Name) (objectiveID :type Name))
  (returns (`Completed?` :type Boolean))
  (locals (TempObjectives :type "Array of /Game/QuestSystem/Structs/S_QuestObjective Structure"))
  (for (_array_element _array_index) (`self.ActiveQuests`)
    (bind ((`QuestID_15_822500384463595D74E8C3A0EFD088AB` _questid) (`Objectives_20_897191804E9E5A681C401483E0AEB55B` _objectives)) (break `/Game/QuestSystem/Structs/S_QuestData` _array_element))
    (set `local.TempObjectives` _objectives)
    (if (== _questid QuestID)
      (for (_array_element_2 _array_index_2) (`.Objectives_20_897191804E9E5A681C401483E0AEB55B` (break `/Game/QuestSystem/Structs/S_QuestData` _array_element))
        (if (== (`.ObjectiveID_5_E318AE8B44FE4C490F23A1996DC67BF0` (break `/Game/QuestSystem/Structs/S_QuestObjective` _array_element_2)) objectiveID)
          (bind (_objectiveid _description _iscompleted _objectivetype _targetdata _optional _cancompleteanyorder_) (break `/Game/QuestSystem/Structs/S_QuestObjective` _array_element_2))
          (`KismetArrayLibrary.Array_Set` (`local.TempObjectives`) _array_index_2 (make `/Game/QuestSystem/Structs/S_QuestObjective` _objectiveid _description true _objectivetype _targetdata _optional _cancompleteanyorder_))
          (bind (_questid_2 _title _description_2 _objectives_2 _isrepitable _autostart _rewards) (break `/Game/QuestSystem/Structs/S_QuestData` _array_element))
          (`KismetArrayLibrary.Array_Set` (`self.ActiveQuests`) _array_index (make `/Game/QuestSystem/Structs/S_QuestData` _questid_2 _title _description_2 (`local.TempObjectives`) _isrepitable _autostart _rewards))
          (bind _completed_ (`self.CheckQuestCompleted` _questid_2))
          (return _completed_)))
      (else
        (return false)))))

(fn `UserConstructionScript`)